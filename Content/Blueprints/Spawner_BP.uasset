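; Spawner actor that toggles periodic spawning of AI Wild Fuzzy actors each time the player's ThirdPersonCharacter begins overlapping its trigger box.
; A FlipFlop alternates between starting a looping Spawn timer and clearing it while destroying every tracked spawn.
; Each spawn lands at a random point around SpawnVolume and is stored in an array.
; The construction script sizes SpawnVolume from the BoxExtent variable.
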(event `self.Box.OnComponentBeginOverlap`
  (params (OverlappedComponent :type "PrimitiveComponent Object Reference") (OtherActor :type "Actor Object Reference") (OtherComp :type "PrimitiveComponent Object Reference") (OtherBodyIndex :type Integer) (bFromSweep :type Boolean) (SweepResult :type "HitResult Structure (by ref)"))
  (cast `/Game/ThirdPersonBP/Blueprints/ThirdPersonCharacter` OtherActor)
  (`/Engine/EditorBlueprintResources/StandardMacros.FlipFlop`
    (:`A`
      (`KismetSystemLibrary.K2_SetTimer` null "Spawn" 3.0 true))
    (:`B`
      (`KismetSystemLibrary.K2_ClearTimer` null "Spawn")
      (for _array_element (`self.Spawned Actor`)
        (`self.K2_DestroyActor` _array_element)))))

(event `Spawn`
  (bind _returnvalue (`|SpawnActorFromClass` "/Game/AI/AI__Wild_Fuzzy.AI__Wild_Fuzzy_C" (`KismetMathLibrary.MakeTransform` (`KismetMathLibrary.RandomPointInBoundingBox` (`SceneComponent.K2_GetComponentLocation` (`self.SpawnVolume`)) (`self.Box Extent`))) "Undefined" "OverrideRootScale" null null))
  (`KismetArrayLibrary.Array_Add` (`self.Spawned Actor`) _returnvalue))

(fn `UserConstructionScript`
  (`BoxComponent.SetBoxExtent` (`self.SpawnVolume`) (`self.Box Extent`) true))
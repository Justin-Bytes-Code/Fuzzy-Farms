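; Carrot_BP is a food pickup that spins in place and can be collected with the Interact input.
; Tick rotates the Cube around its yaw at Speed, scaled by delta time.
; Any overlap with the Box enables input from player controller 0, which is never disabled afterward.
; Pressing Interact then plays the Camera_Shutter sound in 2D and destroys the actor.
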(event `self.ReceiveBeginPlay`)

(event `self.ReceiveTick`
  (params (DeltaSeconds :type "Float (single-precision)"))
  ;[1 1 1] Make the Food rotate
  (`SceneComponent.K2_AddLocalRotation` (`self.Cube`) (* (`KismetMathLibrary.MakeRotator` 0.0 0.0 (`self.Speed`)) DeltaSeconds) false false))

(event `InputAction|Interact`
  (params (Key :type "Key Structure"))
  ;[1 1 1] When Button is pressed it will make object disapper and play a sound
  (:`Pressed`
    (`GameplayStatics.PlaySound2D` "/Engine/VREditor/Sounds/UI/Camera_Shutter.Camera_Shutter" 1.0 1.0 0.0 null null)
    (`self.K2_DestroyActor`)))

(event `self.Box.OnComponentBeginOverlap`
  (params (OverlappedComponent :type "PrimitiveComponent Object Reference") (OtherActor :type "Actor Object Reference") (OtherComp :type "PrimitiveComponent Object Reference") (OtherBodyIndex :type Integer) (bFromSweep :type Boolean) (SweepResult :type "HitResult Structure (by ref)"))
  ;[1 1 1] Enables controller
  (`self.EnableInput` (`GameplayStatics.GetPlayerController` 0)))

(fn `UserConstructionScript`)